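; AI controller for an enemy pawn that switches between three alert states as it detects the Hero.
; Sight through PawnSensing triggers a faster chase to the last known position, and timers step the alert state down.
; Loud enough noise turns the pawn and starts a slower, self-repeating patrol to random points around that last position, or around home if none.
; AIPerception updates only draw debug shapes and text.
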(event `self.ReceiveTick`
  (params (DeltaSeconds :type "Float (single-precision)")))

(event `self.ReceiveBeginPlay`
  (`|ExecutionSequence`
    (:`then_0`
      (set `self.State` "NewEnumerator0"))
    (:`then_1`
      (`KismetSystemLibrary.Delay` 0.5)
      (set `self.HomePostion` (`self.K2_GetActorLocation` (`self.K2_GetPawn`))))
    (:`then_2`
      (`KismetSystemLibrary.Delay` 1.0)
      (set `self.PatrolCount` 0))))

(event `UpdateVelocity`
  (params (NewMaxWalkSpeed :type "Float (double-precision)"))
  (bind _asenemy (cast `/Game/Blueprints/Enemy` (`self.K2_GetPawn`)))
  (`/Game/Blueprints/Enemy.ChangeSpeed` _asenemy NewMaxWalkSpeed))

(event `Patrol`
  (bind _returnvalue (`self.K2_GetPawn`))
  (bind _lastpositionknowed (`self.LastPositionKnowed`))
  (bind _patroldestination (`self.PatrolDestination`))
  (bind (_randomlocation _returnvalue_2) (`NavigationSystemV1.K2_GetRandomReachablePointInRadius` _lastpositionknowed 500.0 null null))
  (bind (_randomlocation_2 _returnvalue_3) (`NavigationSystemV1.K2_GetRandomReachablePointInRadius` (`self.HomePostion`) 2000.0 null null))
  ;[1 1 1] Patrol
  (if (not (`|EnumEquality` (`self.State`) "NewEnumerator2"))
    (cast `/Game/Blueprints/Enemy` (`self.K2_GetPawn`))
    (`self.updateVelocity` 200.0)
    (if (!= _lastpositionknowed (0.0 0.0 0.0))
      (set `self.PatrolDestination` _randomlocation)
      (if _returnvalue_2
        (`|AIMoveTo` _returnvalue _patroldestination null :!label _label
          (:`OnSuccess`
            _))
        (else
          (`|AIMoveTo` _returnvalue _patroldestination null :!label _label_2
            (:`OnSuccess`
              _))))
      (else
        (set `self.PatrolDestination` _randomlocation_2)
        (if _returnvalue_3
          (goto _label)
          (else
            (goto _label_2)))))
    (`/Engine/EditorBlueprintResources/StandardMacros.IncrementInt` (`self.PatrolCount`)
      (:`  `
        (if (> (`self.PatrolCount`) 1)
          (set `self.State` "NewEnumerator0"))
        (set `self.PatrolCount` 0)
        (`self.Patrol`)))))

(event `TrackPlayer`
  ;[1 1 1] Alerts
  (if (`|EnumEquality` (`self.State`) "NewEnumerator2")
    (`self.updateVelocity` 300.0)
    (`|AIMoveTo` (`self.K2_GetPawn`) (`self.LastPositionKnowed`) null
      (:`then`
        _)
      (:`OnSuccess`
        _))
    (`KismetSystemLibrary.K2_ClearTimer` null "ResetAlerts")
    (`KismetSystemLibrary.K2_SetTimer` null "ResetAlerts" 0.3)))

(event `self.PawnSensing.OnSeePawn`
  (params (Pawn :type "Pawn Object Reference"))
  (set `self.State` "NewEnumerator2")
  (set `self.LastPositionKnowed` (`self.K2_GetActorLocation` (cast `/Game/Blueprints/Hero` Pawn :!pure true)))
  (`self.TrackPlayer`))

(event `ResetAlerts`
  ;[1 1 1] Reset to Idle
  (if (`|EnumEquality` (`self.State`) "NewEnumerator2")
    (set `self.State` "NewEnumerator1")
    (else
      (set `self.State` "NewEnumerator0"))))

(event `self.PawnSensing.OnHearNoise`
  (params (Instigator :type "Pawn Object Reference") (Location :type "Vector Structure (by ref)") (Volume :type "Float (single-precision)"))
  (bind _returnvalue (`self.K2_GetPawn`))
  (if (not (`|EnumEquality` (`self.State`) "NewEnumerator2"))
    (cast `/Game/Blueprints/Hero` Instigator)
    (if (>= Volume 0.5)
      (set `self.State` "NewEnumerator1")
      (`|ExecutionSequence`
        (:`then_0`
          (bind _returnvalue_2 (`self.K2_SetActorRotation` _returnvalue (`KismetMathLibrary.RLerp` (`self.K2_GetActorRotation` _returnvalue) (`KismetMathLibrary.FindLookAtRotation` (`self.K2_GetActorLocation` _returnvalue) Location) 0.1) false))
          (if _returnvalue_2
            (`self.Patrol`)
            (`KismetSystemLibrary.K2_ClearTimer` null "ResetAlerts")
            (`KismetSystemLibrary.K2_SetTimer` null "ResetAlerts" 1.0)))))))

(event `self.AIPerception.OnTargetPerceptionUpdated`
  (params (Actor :type "Actor Object Reference") (Stimulus :type "AIStimulus Structure"))
  (bind (_age _expirationage _strength _stimuluslocation _receiverlocation) (break `AIStimulus` Stimulus))
  (cast `/Game/Blueprints/Hero` Actor
    (:`then`
      (`KismetSystemLibrary.DrawDebugSphere` _stimuluslocation 100.0 12 (struct :`R` 0.512153 :`G` 0.460666 :`B` 0.012056 :`A` 0.997) 1.0 1.0))
    (:`CastFailed`
      (`KismetSystemLibrary.DrawDebugString` _receiverlocation "Idle or not hearin / seeing nothing" null (struct :`R` 0.618055 :`G` 0.069118 :`A` 1.0) 2.0))))

(fn `UserConstructionScript`)