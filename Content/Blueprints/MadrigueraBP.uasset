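; MadrigueraBP is a destructible burrow that spawns enemies and can be destroyed by the Hero.
; SpawnEnemy, not called within this Blueprint, spawns an AI at a random point in SpawnVolume while the world count of that class is at most MaxEnemy.
; Hero damage is added to clamped health, so only negative values reduce it.
; At zero health it plays explosion and collapse effects, then destroys itself after a short delay.
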(event `self.ReceiveBeginPlay`
  (set `self.HealthMadriguera` (`self.MaxHealth`)))

(event `SpawnEnemy`
  (bind _spawnvolume (`self.SpawnVolume`))
  (bind _outactors (`GameplayStatics.GetAllActorsOfClass` "/Game/Blueprints/Enemy.Enemy_C")) ; Crear Clase Padre
  (if (<= (`KismetArrayLibrary.Array_Length` _outactors) (`self.MaxEnemy`))
    (`AIBlueprintHelperLibrary.SpawnAIFromClass` "/Game/Blueprints/Enemy.Enemy_C" null (`KismetMathLibrary.RandomPointInBoundingBox` (`SceneComponent.K2_GetComponentLocation` _spawnvolume) (`BoxComponent.GetScaledBoxExtent` _spawnvolume)) (struct) false null)))

(event `self.ReceiveAnyDamage`
  (params (Damage :type "Float (single-precision)") (DamageType :type "DamageType Object Reference") (InstigatedBy :type "Controller Object Reference") (DamageCauser :type "Actor Object Reference"))
  (bind _returnvalue (`SceneComponent.K2_GetComponentLocation` (`self.StaticMesh`)))
  (cast `/Game/Blueprints/Hero` DamageCauser)
  (`self.Calcule Health` Damage)
  (`self.CalculeDead`)
  (if (`self.Death`)
    (`GameplayStatics.SpawnEmitterAtLocation` "/Game/StarterContent/Particles/P_Explosion.P_Explosion" _returnvalue)
    (`GameplayStatics.SpawnSoundAtLocation` "/Game/StarterContent/Audio/Collapse_Cue.Collapse_Cue" _returnvalue (struct) 1.0 1.0 0.0 null null)
    (`KismetSystemLibrary.Delay` 0.5)
    (`self.K2_DestroyActor`)))

(fn `Calcule Health`
  (params (Delta :type "Float (double-precision)"))
  (set `self.HealthMadriguera` (`KismetMathLibrary.FClamp` (+ Delta (`self.HealthMadriguera`)) 0.0 (`self.MaxHealth`))))

(fn `CalculeDead`
  (if (<= (`self.HealthMadriguera`) 0.0)
    (set `self.Death` true)))

(fn `GetHealth`
  (returns (HealthMadriguera :type "Float (double-precision)"))
  (return (`self.HealthMadriguera`)))

(fn `GetHealth_Percentil`
  (returns (HealthMadriguera :type "Float (double-precision)"))
  (return (/ (`self.HealthMadriguera`) (`self.MaxHealth`))))

(fn `UserConstructionScript`)