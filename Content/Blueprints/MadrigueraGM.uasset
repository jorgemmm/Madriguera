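; MadrigueraGM is a game mode Blueprint that drives enemy spawning and hero respawning.
; On BeginPlay it caches the PlayerStarts and sets a looping SpawnEnemy timer on every MadrigueraBP, at an interval derived from SpawnSpeed.
; RespawnPlayer waits through a delay, spawns a new Hero at the first PlayerStart and has player controller 0 possess it.
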(event `self.ReceiveBeginPlay`
  (`|ExecutionSequence`
    (:`then_0`
      (bind _outactors (`GameplayStatics.GetAllActorsOfClass` "/Script/Engine.PlayerStart"))
      (set `self.PlayerStarts` _outactors))
    (:`then_1`
      (bind _outactors_2 (`GameplayStatics.GetAllActorsOfClass` "/Game/Blueprints/MadrigueraBP.MadrigueraBP_C"))
      (for _array_element _outactors_2
        (`KismetSystemLibrary.K2_SetTimer` _array_element "SpawnEnemy" (/ 1.0 (`self.SpawnSpeed`)) true)))))

(event `RespawnPlayer`
  (`|ExecutionSequence`
    (:`then_1`
      (`KismetSystemLibrary.Delay` 5.0)
      (bind _returnvalue (`|SpawnActorFromClass` "/Game/Blueprints/Hero.Hero_C" (`self.GetTransform` (`|GetArrayItem` (`self.PlayerStarts`))) "Undefined" "OverrideRootScale" null null)) ; P
      (`Controller.Possess` (`GameplayStatics.GetPlayerController` 0) _returnvalue))))

(fn `UserConstructionScript`)